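; BP_NextLevel is a level-exit trigger that lets the player press F inside its box to advance to the next level.
; Box overlap with the player enables or disables input and opens or closes a gate that guards the F key.
; On F, it copies the character's puzzle (Pintu) flags, Count and Over flags into the youxishili game instance through Saves.
; It then picks the next level by current name, chaining DANYUAN1 through DANYUAN5 and ending at 拼图关卡.
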(event `Key|F`
  (params (Key :type "Key Structure"))
  (:`Pressed`
    (`/Engine/EditorBlueprintResources/StandardMacros.Gate` true :!label _label
      (:`Exit`
        (`|ExecutionSequence`
          (:`then_0`
            (bind _asbp_first_person_character (cast `/Game/FirstPerson/Blueprints/BP_FirstPersonCharacter` (`GameplayStatics.GetPlayerCharacter` 0)))
            (bind _asyouxishili (cast `/Game/FirstPerson/GameMode/youxishili` (`GameplayStatics.GetGameInstance`)))
            (`/Game/FirstPerson/GameMode/youxishili.Saves` _asyouxishili (`/Game/FirstPerson/Blueprints/BP_FirstPersonCharacter.pintu1isok` _asbp_first_person_character) (`/Game/FirstPerson/Blueprints/BP_FirstPersonCharacter.pintu2isok` _asbp_first_person_character) (`/Game/FirstPerson/Blueprints/BP_FirstPersonCharacter.pintu3isok` _asbp_first_person_character) (`/Game/FirstPerson/Blueprints/BP_FirstPersonCharacter.pintu4isok` _asbp_first_person_character) (`/Game/FirstPerson/Blueprints/BP_FirstPersonCharacter.count` _asbp_first_person_character) (`/Game/FirstPerson/Blueprints/BP_FirstPersonCharacter.over1` _asbp_first_person_character) (`/Game/FirstPerson/Blueprints/BP_FirstPersonCharacter.over2` _asbp_first_person_character) (`/Game/FirstPerson/Blueprints/BP_FirstPersonCharacter.over3` _asbp_first_person_character) (`/Game/FirstPerson/Blueprints/BP_FirstPersonCharacter.over4` _asbp_first_person_character) (`/Game/FirstPerson/Blueprints/BP_FirstPersonCharacter.over5` _asbp_first_person_character)))
          (:`then_1`
            (bind _returnvalue (`GameplayStatics.GetCurrentLevelName` true))
            (if (`KismetStringLibrary.EqualEqual_StrStr` _returnvalue "DANYUAN1")
              (`GameplayStatics.OpenLevelBySoftObjectPtr` "/Game/MAP/DANYUAN2.DANYUAN2")
              (elif (`KismetStringLibrary.EqualEqual_StrStr` _returnvalue "DANYUAN2")
                (`GameplayStatics.OpenLevelBySoftObjectPtr` "/Game/MAP/DANYUAN3.DANYUAN3")
                (elif (`KismetStringLibrary.EqualEqual_StrStr` _returnvalue "DANYUAN3")
                  (`GameplayStatics.OpenLevelBySoftObjectPtr` "/Game/MAP/DANYUAN4.DANYUAN4")
                  (elif (`KismetStringLibrary.EqualEqual_StrStr` _returnvalue "DANYUAN4")
                    (`GameplayStatics.OpenLevelBySoftObjectPtr` "/Game/MAP/DANYUAN5.DANYUAN5")
                    (elif (`KismetStringLibrary.EqualEqual_StrStr` _returnvalue "DANYUAN5")
                      (`GameplayStatics.OpenLevelBySoftObjectPtr` "/Game/MAP/拼图关卡.拼图关卡"))))))))))))

(event `self.Box.OnComponentBeginOverlap`
  (params (OverlappedComponent :type "PrimitiveComponent Object Reference") (OtherActor :type "Actor Object Reference") (OtherComp :type "PrimitiveComponent Object Reference") (OtherBodyIndex :type Integer) (bFromSweep :type Boolean) (SweepResult :type "HitResult Structure (by ref)"))
  (if (== OtherActor (`GameplayStatics.GetPlayerCharacter` 0))
    (`self.EnableInput` (`GameplayStatics.GetPlayerController` 0))
    (goto _label :!via `Open`)))

(event `self.Box.OnComponentEndOverlap`
  (params (OverlappedComponent :type "PrimitiveComponent Object Reference") (OtherActor :type "Actor Object Reference") (OtherComp :type "PrimitiveComponent Object Reference") (OtherBodyIndex :type Integer))
  (if (== OtherActor (`GameplayStatics.GetPlayerCharacter` 0))
    (`self.DisableInput` (`GameplayStatics.GetPlayerController` 0))
    (goto _label :!via `Close`)))

(fn `UserConstructionScript`)