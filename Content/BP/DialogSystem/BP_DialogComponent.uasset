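; BP_DialogComponent is a dialog component that shows and closes a dialog UI from its stored dialog struct.
; OpenDialog creates a WP_DialogInterFace widget, adds it to the viewport, shows the mouse cursor, passes in the name, content and image, then calls the widget's Dialog function.
; OverDialog removes that widget and any top-level widgets of the same class, but leaves the cursor setting unchanged.
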(event `OpenDialog`
  (bind _dialogui (`self.DialogUI`))
  (bind (_name _content _img) (break `/Game/BP/DialogSystem/ST_DialogStruct` (`self.DIalogStruct`)))
  (bind _returnvalue (`|CreateWidget` "/Game/BP/DialogSystem/WP_DialogInterFace.WP_DialogInterFace_C"))
  (bind _output_get (set `self.DialogUI` _returnvalue))
  (`UserWidget.AddToViewport` _output_get 0)
  (set `PlayerController.bShowMouseCursor` true (`GameplayStatics.GetPlayerController` 0))
  (set `/Game/BP/DialogSystem/WP_DialogInterFace.Value` (make `/Game/BP/DialogSystem/ST_DialogStruct` _name _content _img) _dialogui)
  (`/Game/BP/DialogSystem/WP_DialogInterFace.Dialog` _dialogui))

(event `OverDialog`
  (`Widget.RemoveFromParent` (`self.DialogUI`))
  (bind _foundwidgets (`WidgetBlueprintLibrary.GetAllWidgetsOfClass` "/Game/BP/DialogSystem/WP_DialogInterFace.WP_DialogInterFace_C"))
  (`Widget.RemoveFromParent` _foundwidgets))