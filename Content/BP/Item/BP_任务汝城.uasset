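; Interactable task exhibit (任务汝城) that shows its information and advances the player from Task1 to Task2.
; BeginPlay loads the exhibit's row from Zhanpin_DataTable by its ItemName enum.
; Sphere gates F input, which opens the info widget and plays WP_Guide, then advances WP_TaskInterFace once if Task1 is set.
; During Task1, Sphere1 hides the camera-facing marker widget and shows a one-time F prompt, removed on exit.
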(event `self.ReceiveBeginPlay`
  (bind _asbp_first_person_character (cast `/Game/FirstPerson/Blueprints/BP_FirstPersonCharacter` (`GameplayStatics.GetPlayerCharacter` 0)))
  (set `self.Player` _asbp_first_person_character)
  (bind _returnvalue (`|GetDataTableRow` "/Game/BP/Item/zhanpin_DataTable.zhanpin_DataTable" (`KismetStringLibrary.Conv_StringToName` (`|GetEnumeratorNameAsString` (`self.ItemName`))))
    (:`then`
      (set `self.Itemproperty` _returnvalue))))

(event `Key|F`
  (params (Key :type "Key Structure"))
  (bind _player (`self.Player`))
  (bind (_name _jianlue _xiangxi _img) (break `/Game/BP/Item/zhanpin` (`self.Itemproperty`)))
  (:`Pressed`
    (`/Engine/EditorBlueprintResources/StandardMacros.Gate` true :!label _label
      (:`Exit`
        (`|ExecutionSequence`
          (:`then_0`
            (if (not (`self.Create?`))
              (bind _returnvalue (`|CreateWidget` "/Game/UMG/AI_Guide/WP_ZhanpinXinxi.WP_ZhanpinXinxi_C"))
              (set `TextBlock.Text` (`KismetTextLibrary.Conv_StringToText` _jianlue) (`/Game/UMG/AI_Guide/WP_ZhanpinXinxi.jianlue` _returnvalue))
              (set `Image.Brush` (make `SlateBrush` "Image" "NoTile" "NoMirror" (struct :`X` 32.0 :`Y` 32.0) (struct) (struct :`SpecifiedColor` (struct :`R` 1.0 :`G` 1.0 :`B` 1.0 :`A` 1.0) :`ColorUseRule` "UseColor_Specified") (struct :`CornerRadii` (struct) :`Color` (struct :`SpecifiedColor` (struct) :`ColorUseRule` "UseColor_Specified") :`RoundingType` "HalfHeightRadius") _img) (`/Game/UMG/AI_Guide/WP_ZhanpinXinxi.img` _returnvalue))
              (set `TextBlock.Text` (`KismetTextLibrary.Conv_NameToText` _name) (`/Game/UMG/AI_Guide/WP_ZhanpinXinxi.name` _returnvalue))
              (bind _foundwidgets (`WidgetBlueprintLibrary.GetAllWidgetsOfClass` "/Game/UMG/AI_Guide/WP_Guide.WP_Guide_C"))
              (`Widget.RemoveFromParent` _foundwidgets)
              (bind _returnvalue_2 (`|CreateWidget` "/Game/UMG/AI_Guide/WP_Guide.WP_Guide_C"))
              (set `TextBlock.Text` (`KismetTextLibrary.Conv_StringToText` _xiangxi) (`/Game/UMG/AI_Guide/WP_Guide.content` _returnvalue_2))
              (`UserWidget.AddToViewport` _returnvalue_2 0)
              (`UserWidget.AddToViewport` _returnvalue 0)
              (`/Game/UMG/AI_Guide/WP_Guide.play` _returnvalue_2)))
          (:`then_1`
            (if (`/Game/FirstPerson/Blueprints/BP_FirstPersonCharacter.task1` _player)
              (`/Engine/EditorBlueprintResources/StandardMacros.DoOnce` false
                (:`Completed`
                  (set `/Game/FirstPerson/Blueprints/BP_FirstPersonCharacter.task2` true _player)
                  (bind _foundwidgets_2 (`WidgetBlueprintLibrary.GetAllWidgetsOfClass` "/Game/BP/TaskSystem/WP_TaskInterFace.WP_TaskInterFace_C"))
                  (for _array_element _foundwidgets_2
                    (`/Game/BP/TaskSystem/WP_TaskInterFace.Next Task` _array_element)))))))))))

(event `self.Sphere.OnComponentBeginOverlap`
  (params (OverlappedComponent :type "PrimitiveComponent Object Reference") (OtherActor :type "Actor Object Reference") (OtherComp :type "PrimitiveComponent Object Reference") (OtherBodyIndex :type Integer) (bFromSweep :type Boolean) (SweepResult :type "HitResult Structure (by ref)"))
  (if (== OtherActor (`GameplayStatics.GetPlayerCharacter` 0))
    (`self.EnableInput` (`GameplayStatics.GetPlayerController` 0))
    (goto _label :!via `Open`)))

(event `self.Sphere.OnComponentEndOverlap`
  (params (OverlappedComponent :type "PrimitiveComponent Object Reference") (OtherActor :type "Actor Object Reference") (OtherComp :type "PrimitiveComponent Object Reference") (OtherBodyIndex :type Integer))
  (if (== OtherActor (`GameplayStatics.GetPlayerCharacter` 0))
    (`self.DisableInput` (`GameplayStatics.GetPlayerController` 0))
    (goto _label :!via `Close`)))

(event `self.Sphere1.OnComponentBeginOverlap`
  (params (OverlappedComponent :type "PrimitiveComponent Object Reference") (OtherActor :type "Actor Object Reference") (OtherComp :type "PrimitiveComponent Object Reference") (OtherBodyIndex :type Integer) (bFromSweep :type Boolean) (SweepResult :type "HitResult Structure (by ref)"))
  (cast `/Game/FirstPerson/Blueprints/BP_FirstPersonCharacter` OtherActor)
  (if (`/Game/FirstPerson/Blueprints/BP_FirstPersonCharacter.task1` (`self.Player`))
    (`SceneComponent.SetVisibility` (`self.Widget`) false false)
    (if (not (`self.F_TipsIsCreate?`))
      (`/Engine/EditorBlueprintResources/StandardMacros.DoOnce` false
        (:`Completed`
          (bind _returnvalue (`|CreateWidget` "/Game/BP/DialogSystem/WP_Tip_F.WP_Tip_F_C"))
          (`UserWidget.AddToViewport` _returnvalue 0)
          (set `self.F_TipsIsCreate?` true))))))

(event `self.Sphere1.OnComponentEndOverlap`
  (params (OverlappedComponent :type "PrimitiveComponent Object Reference") (OtherActor :type "Actor Object Reference") (OtherComp :type "PrimitiveComponent Object Reference") (OtherBodyIndex :type Integer))
  (if (`self.F_TipsIsCreate?`)
    (if (`KismetSystemLibrary.IsValid` (stale `self.Sphere1.OnComponentBeginOverlap` _returnvalue))
      (bind _foundwidgets (`WidgetBlueprintLibrary.GetAllWidgetsOfClass` "/Game/BP/DialogSystem/WP_Tip_F.WP_Tip_F_C"))
      (`Widget.RemoveFromParent` _foundwidgets)
      (set `self.F_TipsIsCreate?` false))))

(event `self.ReceiveTick`
  (params (DeltaSeconds :type "Float (single-precision)"))
  (`SceneComponent.K2_SetWorldRotation` (`self.Widget`) (`KismetMathLibrary.FindLookAtRotation` (`SceneComponent.K2_GetComponentLocation` (`self.Widget`)) (`PlayerCameraManager.GetCameraLocation` (`GameplayStatics.GetPlayerCameraManager` 0))) false false))

(fn `UserConstructionScript`)